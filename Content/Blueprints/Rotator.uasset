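; Rotator actor that turns one layer of a Rubik's-style cube (RCube) in quarter steps and is destroyed along with it.
; Cuboids overlapping its Box are attached to it, then the Box yaws by animated Timeline or instantly, blocked while RCube is rotating unless forced.
; After each turn it checks the faces, clearing the move string if solved.
; Otherwise it looks up the state in RCube's States map, logging the axis-indexed move for new states.
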(event `self.ReceiveBeginPlay`
  (add `self.OnDestroyed` (`self.RCube`) (delegate `OnDestroyed_Event_0`)))

(event `OnDestroyed_Event_0` :!signature `self.OnDestroyed`
  (params (DestroyedActor :type "Actor Object Reference"))
  (`self.K2_DestroyActor`))

(event `Rotate`
  (params (`Reverse?` :type Boolean) (Rate :type "Float (single-precision)" :default 1.0) (Force :type Boolean))
  (bind _rcube (`self.RCube`))
  (bind _rcube_2 (`self.RCube`))
  (bind _rcube_3 (`self.RCube`))
  (bind (_return_state _solved) (`/Game/Blueprints/RCube.Check Faces` _rcube))
  (bind _statemoves (`/Game/Blueprints/RCube.StateMoves` _rcube))
  (bind _states (`/Game/Blueprints/RCube.States` _rcube))
  (bind (_value _returnvalue) (`BlueprintMapLibrary.Map_Find` _states _return_state))
  (if (`/Game/Blueprints/RCube.Rotating` _rcube_3)
    (if Force
      (`TimelineComponent.SetPlayRate` (`self.Timeline_0`) Rate :!label _label)
      (set `self.Reverse?` `Reverse?`)
      (set `/Game/Blueprints/RCube.Rotating` true _rcube_3)
      (`self.SetParents`)
      (bind _output_get (set `self.Relative Rotation` (`SceneComponent.RelativeRotation` (`self.Box`))))
      (bind (_direction _alpha) (`Timeline|Timeline_0` :!via `PlayFromStart`)
        (:`Update`
          (`SceneComponent.K2_SetRelativeRotation` (`self.Box`) (`KismetMathLibrary.RLerp` _output_get (`KismetMathLibrary.MakeRotator` 0.0 0.0 (`KismetMathLibrary.Conv_IntToDouble` (* (`KismetMathLibrary.Conv_ByteToInt` (`self.NextRState`)) 90))) _alpha true) false false))
        (:`Finished`
          (set `/Game/Blueprints/RCube.Rotating` false (`self.RCube`))
          (set `self.RState` (`self.NextRState`))
          (if _solved
            (set `/Game/Blueprints/RCube.Current State` _return_state (`self.RCube`))
            (set `/Game/Blueprints/RCube.StateMoves` "" (`self.RCube`))
            (else
              (bind _output_get_2 (set `/Game/Blueprints/RCube.Current State` _return_state (`self.RCube`)))
              (if _returnvalue
                (set `/Game/Blueprints/RCube.StateMoves` _value _rcube_2)
                (else
                  (bind _output_get_3 (set `/Game/Blueprints/RCube.StateMoves` (`KismetStringLibrary.Concat_StrStr` _statemoves (`KismetMathLibrary.SelectString` "," "" (> (`KismetStringLibrary.Len` _statemoves) 0)) (`KismetStringLibrary.Concat_StrStr` (`KismetMathLibrary.SelectString` "T" "F" (`self.Reverse?`)) (`.ReturnValue` (`self.FindRotator`)))) _rcube_2))
                  (`BlueprintMapLibrary.Map_Add` _states _output_get_2 _output_get_3))))))))
    (else
      (goto _label))))

(fn `FindRotator`
  (returns (Found :type Boolean) (ReturnValue :type String))
  (bind _rcube (`self.RCube`))
  (bind _returnvalue (`KismetArrayLibrary.Array_Find` (`/Game/Blueprints/RCube.ZRotator` _rcube) self))
  (bind _returnvalue_2 (`KismetArrayLibrary.Array_Find` (`/Game/Blueprints/RCube.XRotators` _rcube) self))
  (bind _returnvalue_3 (`KismetArrayLibrary.Array_Find` (`/Game/Blueprints/RCube.YRotators` _rcube) self))
  (if (> _returnvalue_2 -1)
    (return true (`KismetStringLibrary.Concat_StrStr` "X" (`KismetStringLibrary.Conv_IntToString` _returnvalue_2)))
    (elif (> _returnvalue_3 -1)
      (return true (`KismetStringLibrary.Concat_StrStr` "Y" (`KismetStringLibrary.Conv_IntToString` _returnvalue_3)))
      (elif (> _returnvalue -1)
        (return true (`KismetStringLibrary.Concat_StrStr` "Z" (`KismetStringLibrary.Conv_IntToString` _returnvalue)))
        (else
          (return false ""))))))

(fn `InstantRotate`
  (params (`Reverse?` :type Boolean) (Force :type Boolean))
  (bind _rcube (`self.RCube`))
  (bind _rcube_2 (`self.RCube`))
  (bind _rcube_3 (`self.RCube`))
  (bind (_return_state _solved) (`/Game/Blueprints/RCube.Check Faces` _rcube))
  (bind _statemoves (`/Game/Blueprints/RCube.StateMoves` _rcube))
  (bind _states (`/Game/Blueprints/RCube.States` _rcube))
  (bind (_value _returnvalue) (`BlueprintMapLibrary.Map_Find` _states _return_state))
  (if (`/Game/Blueprints/RCube.Rotating` _rcube_3)
    (if Force
      (set `self.Reverse?` `Reverse?` :!label _label)
      (set `/Game/Blueprints/RCube.Rotating` true _rcube_3)
      (`self.SetParents`)
      (set `self.Relative Rotation` (`SceneComponent.RelativeRotation` (`self.Box`)))
      (`SceneComponent.K2_SetRelativeRotation` (`self.Box`) (`KismetMathLibrary.MakeRotator` 0.0 0.0 (`KismetMathLibrary.Conv_IntToDouble` (* (`KismetMathLibrary.Conv_ByteToInt` (`self.NextRState`)) 90))) false false)
      (set `/Game/Blueprints/RCube.Rotating` false (`self.RCube`))
      (set `self.RState` (`self.NextRState`))
      (if _solved
        (set `/Game/Blueprints/RCube.Current State` _return_state (`self.RCube`))
        (set `/Game/Blueprints/RCube.StateMoves` "" (`self.RCube`))
        (else
          (bind _output_get (set `/Game/Blueprints/RCube.Current State` _return_state (`self.RCube`)))
          (if _returnvalue
            (set `/Game/Blueprints/RCube.StateMoves` (`KismetMathLibrary.SelectString` _value _output_get (> (`KismetStringLibrary.Len` _value) (`KismetStringLibrary.Len` _output_get))) _rcube_2)
            (else
              (bind _output_get_2 (set `/Game/Blueprints/RCube.StateMoves` (`KismetStringLibrary.Concat_StrStr` _statemoves (`KismetMathLibrary.SelectString` "," "" (> (`KismetStringLibrary.Len` _statemoves) 0)) (`KismetStringLibrary.Concat_StrStr` (`KismetMathLibrary.SelectString` "T" "F" (`self.Reverse?`)) (`.ReturnValue` (`self.FindRotator`)))) _rcube_2))
              (`BlueprintMapLibrary.Map_Add` _states _output_get _output_get_2))))))
    (else
      (goto _label))))

(fn `NextRState`
  (returns (ReturnValue :type "/Game/Blueprints/E_RotationState Enum"))
  (bind _rstate (`self.RState`))
  (return (select `bool` (`self.Reverse?`) :`false` (select `/Game/Blueprints/E_RotationState` _rstate :`NewEnumerator0` "NewEnumerator1" :`NewEnumerator1` "NewEnumerator2" :`NewEnumerator2` "NewEnumerator3" :`NewEnumerator3` "NewEnumerator0" :!type "/Game/Blueprints/E_RotationState Enum") :`true` (select `/Game/Blueprints/E_RotationState` _rstate :`NewEnumerator0` "NewEnumerator3" :`NewEnumerator1` "NewEnumerator0" :`NewEnumerator2` "NewEnumerator1" :`NewEnumerator3` "NewEnumerator2" :!type "/Game/Blueprints/E_RotationState Enum"))))

(fn `SetParents`
  (for _array_element (`PrimitiveComponent.GetOverlappingActors` (`self.Box`) "/Game/Blueprints/Cuboid.Cuboid_C")
    (`self.K2_AttachToComponent` _array_element (`self.Box`) "None" "KeepWorld" "KeepWorld" "KeepWorld" true)))

(fn `UserConstructionScript`)