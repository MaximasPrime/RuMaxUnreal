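; GI_Cube, by its name the Game Instance, starts a new game around a configurable RCube pawn.
; StartNewGame destroys any existing player pawn, adds a new HUD widget to the viewport and masks the view with a timed solid-black camera fade.
; It then spawns an RCube with its stored Dimension and Colours, has the player controller possess it and calls its Init.
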(event `Start New Game`
  (bind _returnvalue (`GameplayStatics.GetPlayerPawn` 0))
  (`/Engine/EditorBlueprintResources/StandardMacros.IsValid` _returnvalue
    (:`Is Valid`
      (`Actor.K2_DestroyActor` _returnvalue))
    (:`Is Not Valid`
      _))
  (bind _returnvalue_2 (`|CreateWidget` "/Game/Widgets/HUD.HUD_C"))
  (`UserWidget.AddToViewport` _returnvalue_2 0)
  (`PlayerCameraManager.StartCameraFade` (`PlayerController.PlayerCameraManager` (`GameplayStatics.GetPlayerController` 0)) 1.0 1.0 5.0 (struct :`A` 1.0) false false)
  (bind _returnvalue_3 (`|SpawnActorFromClass` "/Game/Blueprints/RCube.RCube_C" (`KismetMathLibrary.MakeTransform` (0.0 0.0 0.0)) "Undefined" "OverrideRootScale" null (`self.Dimension`) (`self.Colours`) null))
  (`Controller.Possess` (`GameplayStatics.GetPlayerController` 0) _returnvalue_3)
  (`/Game/Blueprints/RCube.Init` _returnvalue_3))