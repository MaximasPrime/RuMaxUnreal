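; Player-controlled Rubik's cube puzzle of configurable Dimension, with orbit camera, random scrambling and per-size saving of States.
; On BeginPlay it spawns a Rotator per layer on each axis, outer-shell Cuboids and six face boxes that read state and solved status.
; Mouse drags find the Rotator overlapping both start and end pieces, then rotate it on release.
; Solve plays the StateMoves string back from last to first through those Rotators.
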(event `InputAction|Click`
  (params (Key :type "Key Structure"))
  (bind _common_rotator (`self.Common Rotator`))
  (bind (_locationx _locationy) (`WidgetLayoutLibrary.GetMousePositionScaledByDPI` (`GameplayStatics.GetPlayerController` 0)))
  (bind (_bblockinghit _binitialoverlap _time _distance _location _impactpoint _normal _impactnormal _physmat _hitactor _hitcomponent) (`GameplayStatics.BreakHitResult` (`PlayerController.GetHitResultUnderCursorByChannel` (`GameplayStatics.GetPlayerController` 0) "TraceTypeQuery1" true)))
  (bind _returnvalue (`SceneComponent.K2_GetComponentLocation` (`Actor.RootComponent` _common_rotator)))
  ;[1 1 1] Really messy needs redoing
  (:`Pressed`
    (set `self.End` null)
    (set `self.Common Rotator` null)
    (if (`self.Rotating`)
      _
      (elif _bblockinghit
        (bind _returnvalue_2 (`KismetSystemLibrary.K2_SetTimerDelegate` (delegate `Check next cube`) 0.001 true))
        (set `self.Click handle` _returnvalue_2)
        (set `self.Start` _hitcomponent)
        (set `self.Temp Mouse` (`KismetMathLibrary.MakeVector2D` _locationx _locationy)))))
  (:`Released`
    (if (`KismetSystemLibrary.K2_IsValidTimerHandle` (`self.Click handle`))
      (`KismetSystemLibrary.K2_ClearAndInvalidateTimerHandle` (`self.Click handle`))
      (bind _common_rotator_2 (`self.Common Rotator`)
        (:`then`
          (`/Game/Blueprints/Rotator.Rotate` _common_rotator_2 (> (`KismetMathLibrary.VSize` (- (`SceneComponent.GetUpVector` (`Actor.RootComponent` _common_rotator)) (`KismetMathLibrary.Normal` (`KismetMathLibrary.Cross_VectorVector` (- (`SceneComponent.K2_GetComponentLocation` (`self.Start`)) _returnvalue) (- (`SceneComponent.K2_GetComponentLocation` (`self.End`)) _returnvalue))))) 0.01) 3.0 false)
          (`/Engine/EditorBlueprintResources/StandardMacros.IncrementInt` (`self.Moves`)))
        (:`else`)))))

(event `Check next cube`
  (bind _common_rotator (`self.Common Rotator`))
  (bind (_locationx _locationy) (`WidgetLayoutLibrary.GetMousePositionScaledByDPI` (`GameplayStatics.GetPlayerController` 0)))
  (bind (_bblockinghit _binitialoverlap _time _distance _location _impactpoint _normal _impactnormal _physmat _hitactor _hitcomponent) (`GameplayStatics.BreakHitResult` (`PlayerController.GetHitResultUnderCursorByChannel` (`GameplayStatics.GetPlayerController` 0) "TraceTypeQuery1" true)))
  (bind _returnvalue (`SceneComponent.K2_GetComponentLocation` (`Actor.RootComponent` _common_rotator)))
  (bind (_returnvalue_x _returnvalue_y) (`KismetMathLibrary.BreakVector2D` (/ (- (`self.Temp Mouse`) (`KismetMathLibrary.MakeVector2D` _locationx _locationy)) (`WidgetLayoutLibrary.GetViewportSize`))))
  ;[1 1 1] Really messy needs redoing
  (if _bblockinghit
    (if (!= _hitcomponent (`self.Start`))
      (`|ExecutionSequence`
        (:`then_0`
          (`self.End`
            (:`then`)
            (:`else`
              (set `self.End` _hitcomponent))))
        (:`then_1`
          (bind _start (`self.Start`)
            (:`then`
              (bind _end (`self.End`)
                (:`then`
                  (bind (_returnvalue_2 _component) (`self.CommonColliders` (`PrimitiveComponent.GetOverlappingComponents` _start) (`PrimitiveComponent.GetOverlappingComponents` _end)))
                  (if _returnvalue_2
                    (bind _asrotator (cast `/Game/Blueprints/Rotator` (`ActorComponent.GetOwner` _component)))
                    (`self.Common Rotator`
                      (:`then`
                        (`SceneComponent.K2_SetRelativeRotation` (`/Game/Blueprints/Rotator.Box` _common_rotator) (`KismetMathLibrary.MakeRotator` 0.0 0.0 (+ (* (`KismetMathLibrary.Conv_ByteToInt` (`/Game/Blueprints/Rotator.RState` _common_rotator)) 90) (* (`KismetMathLibrary.Abs` (`KismetMathLibrary.SelectFloat` _returnvalue_x _returnvalue_y (`|EnumEquality` (`/Game/Blueprints/Rotator.Axis` _common_rotator) "NewEnumerator2"))) (`KismetMathLibrary.SelectFloat` -90.0 90.0 (> (`KismetMathLibrary.VSize` (- (`SceneComponent.GetUpVector` (`Actor.RootComponent` _common_rotator)) (`KismetMathLibrary.Normal` (`KismetMathLibrary.Cross_VectorVector` (- (`SceneComponent.K2_GetComponentLocation` (`self.Start`)) _returnvalue) (- (`SceneComponent.K2_GetComponentLocation` (`self.End`)) _returnvalue))))) 0.01))))) false false))
                      (:`else`
                        (bind _output_get (set `self.Common Rotator` _asrotator))
                        (`/Game/Blueprints/Rotator.SetParents` _output_get)))))
                (:`else`)))
            (:`else`)))))))

(event `InputAction|Randomize`
  (params (Key :type "Key Structure"))
  (:`Pressed`
    (`self.DisableInput` (`GameplayStatics.GetPlayerController` 0))
    (bind _returnvalue (`KismetSystemLibrary.K2_SetTimer` null "RandomRot" 0.05 true))
    (`KismetSystemLibrary.Delay` 3.0)
    (`KismetSystemLibrary.K2_ClearAndInvalidateTimerHandle` _returnvalue)
    (`self.EnableInput` (`GameplayStatics.GetPlayerController` 0))))

(event `InputAxis|RotateH`
  (params (AxisValue :type "Float (single-precision)"))
  (if (`self.CameraRotate`)
    (`self.AddControllerYawInput` AxisValue)))

(event `InputAction|Rotate`
  (params (Key :type "Key Structure"))
  (bind _returnvalue (`GameplayStatics.GetPlayerController` 0))
  (:`Pressed`
    (set `self.CameraRotate` true)
    (set `PlayerController.bShowMouseCursor` false _returnvalue))
  (:`Released`
    (set `self.CameraRotate` false)
    (set `PlayerController.bShowMouseCursor` true _returnvalue)))

(event `InputAxis|RotateV`
  (params (AxisValue :type "Float (single-precision)"))
  (if (`self.CameraRotate`)
    (`self.AddControllerPitchInput` AxisValue)))

(event `self.ReceiveBeginPlay`
  (bind _dimension (`self.Dimension`))
  (bind _dimension_2 (`self.Dimension`))
  (`|ExecutionSequence`
    (:`then_0`
      ;[1 1 1] Load any save game
      (bind _returnvalue (`GameplayStatics.DoesSaveGameExist` "Cube" _dimension_2))
      (if _returnvalue
        (bind _returnvalue_2 (`GameplayStatics.LoadGameFromSlot` "Cube" _dimension_2))
        (bind _asrsave (cast `/Game/Blueprints/RSave` _returnvalue_2))
        (set `self.States` (`/Game/Blueprints/RSave.States` _asrsave))))
    (:`then_1`
      (`SceneComponent.K2_SetWorldLocation` (`self.SpringArm`) (+ (`SceneComponent.K2_GetComponentLocation` (`self.Scene`)) (* (`self.Size`) (- _dimension 1) 0.5)) false false)
      (`self.Create Cube`)
      (set `SpringArmComponent.TargetArmLength` (`KismetMathLibrary.Conv_IntToDouble` (* _dimension 200)) (`self.SpringArm`))
      (set `PlayerController.bShowMouseCursor` true (`GameplayStatics.GetPlayerController` 0)))))

(event `Create Cube`
  (bind _zrotator (`self.ZRotator`))
  (bind _xrotators (`self.XRotators`))
  (bind _yrotators (`self.YRotators`))
  (bind _size (`self.Size`))
  (bind _size_2 (`self.Size`))
  (bind _returnvalue (`SceneComponent.K2_GetComponentLocation` (`self.Scene`)))
  (bind _returnvalue_2 (- (`self.Dimension`) 1))
  (bind _returnvalue_3 (* (1.0 1.0 0.2) (`self.Dimension`)))
  (bind _returnvalue_4 (* _size (+ (`self.Dimension`) -1) 0.5))
  (bind (_outvec _out_size) (`self.GetAxisVector` "NewEnumerator0" (`self.K2_GetActorLocation` (`|GetArrayItem` _xrotators)) (/ (`self.Size`) -2.0)))
  (bind (_outvec_2 _out_size_2) (`self.GetAxisVector` "NewEnumerator1" (`self.K2_GetActorLocation` (`|GetArrayItem` _yrotators)) (/ (`self.Size`) -2.0)))
  (bind (_outvec_3 _out_size_3) (`self.GetAxisVector` "NewEnumerator2" (`self.K2_GetActorLocation` (`|GetArrayItem` _zrotator)) (/ (`self.Size`) -2.0)))
  (bind (_outvec_4 _out_size_4) (`self.GetAxisVector` "NewEnumerator0" (`self.K2_GetActorLocation` (`|GetArrayItem` _xrotators (`KismetArrayLibrary.Array_LastIndex` _xrotators))) (/ (`self.Size`) 2.0)))
  (bind (_outvec_5 _out_size_5) (`self.GetAxisVector` "NewEnumerator1" (`self.K2_GetActorLocation` (`|GetArrayItem` _yrotators (`KismetArrayLibrary.Array_LastIndex` _yrotators))) (/ (`self.Size`) 2.0)))
  (bind (_outvec_6 _out_size_6) (`self.GetAxisVector` "NewEnumerator2" (`self.K2_GetActorLocation` (`|GetArrayItem` _zrotator (`KismetArrayLibrary.Array_LastIndex` _zrotator))) (/ (`self.Size`) 2.0)))
  (`|ExecutionSequence`
    (:`then_0`
      (for _index (range (`self.Dimension`))
        (bind _returnvalue_5 (`|SpawnActorFromClass` "/Game/Blueprints/Rotator.Rotator_C" (`KismetMathLibrary.MakeTransform` (+ _returnvalue (`KismetMathLibrary.MakeVector` (* _index _size) _returnvalue_4 _returnvalue_4)) (struct :`Pitch` 90.0) _returnvalue_3) "Undefined" "OverrideRootScale" null self "NewEnumerator0" _index null))
        (`KismetArrayLibrary.Array_Add` (`self.XRotators`) _returnvalue_5)
        (bind _returnvalue_6 (`|SpawnActorFromClass` "/Game/Blueprints/Rotator.Rotator_C" (`KismetMathLibrary.MakeTransform` (+ _returnvalue (`KismetMathLibrary.MakeVector` _returnvalue_4 (* _index _size) _returnvalue_4)) (struct :`Roll` 90.0) _returnvalue_3) "Undefined" "OverrideRootScale" null self "NewEnumerator1" _index null))
        (`KismetArrayLibrary.Array_Add` (`self.YRotators`) _returnvalue_6)
        (bind _returnvalue_7 (`|SpawnActorFromClass` "/Game/Blueprints/Rotator.Rotator_C" (`KismetMathLibrary.MakeTransform` (+ _returnvalue (`KismetMathLibrary.MakeVector` _returnvalue_4 _returnvalue_4 (* _index _size))) (struct) _returnvalue_3) "Undefined" "OverrideRootScale" null self "NewEnumerator2" _index null))
        (`KismetArrayLibrary.Array_Add` (`self.ZRotator`) _returnvalue_7)))
    (:`then_1`
      (for _index_2 (range (+ _returnvalue_2 1))
        (for _index_3 (range (+ _returnvalue_2 1))
          (for _index_4 (range (+ _returnvalue_2 1))
            (bind _returnvalue_8 (+ (`SceneComponent.K2_GetComponentLocation` (`self.Scene`)) (`KismetMathLibrary.MakeVector` (* _index_4 _size_2) (* _index_3 _size_2) (* _index_2 _size_2))))
            (if (`self.Outsside?` _returnvalue_8)
              (`|SpawnActorFromClass` "/Game/Blueprints/Cuboid.Cuboid_C" (`KismetMathLibrary.MakeTransform` _returnvalue_8 (struct) (0.98 0.98 0.98)) "Undefined" "OverrideRootScale" null (`self.Colours`) self null))))))
    (:`then_2`
      (`|ExecutionSequence`
        (:`then_0`
          (`|ExecutionSequence`
            (:`then_0`
              (bind _returnvalue_9 (`AddComponent|NODE_AddBoxComponent-0`))
              (`SceneComponent.K2_SetWorldTransform` _returnvalue_9 (`KismetMathLibrary.MakeTransform` _outvec (struct) _out_size) false false)
              (`SceneComponent.K2_AttachToComponent` _returnvalue_9 (`self.Scene`) "None" "KeepWorld" "KeepWorld" "KeepWorld" true)
              (`KismetArrayLibrary.Array_Add` (`self.FaceCheckCollisions`) _returnvalue_9))
            (:`then_1`
              (bind _returnvalue_10 (`AddComponent|NODE_AddBoxComponent-1`))
              (`SceneComponent.K2_SetWorldTransform` _returnvalue_10 (`KismetMathLibrary.MakeTransform` _outvec_4 (struct) _out_size_4) false false)
              (`SceneComponent.K2_AttachToComponent` _returnvalue_10 (`self.Scene`) "None" "KeepWorld" "KeepWorld" "KeepWorld" true)
              (`KismetArrayLibrary.Array_Add` (`self.FaceCheckCollisions`) _returnvalue_10))
            (:`then_2`
              (bind _returnvalue_11 (`AddComponent|NODE_AddBoxComponent-3`))
              (`SceneComponent.K2_SetWorldTransform` _returnvalue_11 (`KismetMathLibrary.MakeTransform` _outvec_2 (struct) _out_size_2) false false)
              (`SceneComponent.K2_AttachToComponent` _returnvalue_11 (`self.Scene`) "None" "KeepWorld" "KeepWorld" "KeepWorld" true)
              (`KismetArrayLibrary.Array_Add` (`self.FaceCheckCollisions`) _returnvalue_11))
            (:`then_3`
              (bind _returnvalue_12 (`AddComponent|NODE_AddBoxComponent-4`))
              (`SceneComponent.K2_SetWorldTransform` _returnvalue_12 (`KismetMathLibrary.MakeTransform` _outvec_5 (struct) _out_size_5) false false)
              (`SceneComponent.K2_AttachToComponent` _returnvalue_12 (`self.Scene`) "None" "KeepWorld" "KeepWorld" "KeepWorld" true)
              (`KismetArrayLibrary.Array_Add` (`self.FaceCheckCollisions`) _returnvalue_12))
            (:`then_4`
              (bind _returnvalue_13 (`AddComponent|NODE_AddBoxComponent-5`))
              (`SceneComponent.K2_SetWorldTransform` _returnvalue_13 (`KismetMathLibrary.MakeTransform` _outvec_3 (struct) _out_size_3) false false)
              (`SceneComponent.K2_AttachToComponent` _returnvalue_13 (`self.Scene`) "None" "KeepWorld" "KeepWorld" "KeepWorld" true)
              (`KismetArrayLibrary.Array_Add` (`self.FaceCheckCollisions`) _returnvalue_13))
            (:`then_5`
              (bind _returnvalue_14 (`AddComponent|NODE_AddBoxComponent-6`))
              (`SceneComponent.K2_SetWorldTransform` _returnvalue_14 (`KismetMathLibrary.MakeTransform` _outvec_6 (struct) _out_size_6) false false)
              (`SceneComponent.K2_AttachToComponent` _returnvalue_14 (`self.Scene`) "None" "KeepWorld" "KeepWorld" "KeepWorld" true)
              (`KismetArrayLibrary.Array_Add` (`self.FaceCheckCollisions`) _returnvalue_14))))
        (:`then_1`
          (set `self.Current State` (`self.Check Faces`)))))))

(event `Solve`
  (params (`Move Duration` :type "Float (single-precision)"))
  (bind _returnvalue (/ 1.0 `Move Duration`))
  (`self.DisableInput` (`GameplayStatics.GetPlayerController` 0))
  (bind _output_get (set `self.Temp ` (`KismetStringLibrary.ParseIntoArray` (`self.StateMoves`) ",")))
  (if (> (`KismetArrayLibrary.Array_Length` _output_get) 0) :!label _label
    (`|ExecutionSequence`
      (:`then_0`
        (bind _returnvalue_2 (`KismetArrayLibrary.Array_LastIndex` _output_get))
        (bind _output (`|GetArrayItem` _output_get _returnvalue_2))
        (switch `string` (`KismetStringLibrary.GetSubstring` _output 1)
          (:`X`
            (bind _returnvalue_3 (`KismetStringLibrary.Conv_StringToInt` (`KismetStringLibrary.Trim` (`KismetStringLibrary.GetSubstring` _output 2 2))))
            (bind _returnvalue_4 (`KismetStringLibrary.EqualEqual_StrStr` (`KismetStringLibrary.GetSubstring` _output) "F"))
            (`/Game/Blueprints/Rotator.Rotate` (`|GetArrayItem` (`self.XRotators`) _returnvalue_3) _returnvalue_4 _returnvalue false))
          (:`Y`
            (`/Game/Blueprints/Rotator.Rotate` (`|GetArrayItem` (`self.YRotators`) _returnvalue_3) _returnvalue_4 _returnvalue false))
          (:`Z`
            (`/Game/Blueprints/Rotator.Rotate` (`|GetArrayItem` (`self.ZRotator`) _returnvalue_3) _returnvalue_4 _returnvalue false))))
      (:`then_1`
        (`KismetArrayLibrary.Array_Remove` _output_get _returnvalue_2)
        (`KismetSystemLibrary.Delay` `Move Duration`)
        (goto _label)))
    (else
      (`self.EnableInput` null))))

(event `Key|K`
  (params (Key :type "Key Structure"))
  (:`Pressed`
    (`self.Solve` 0.5)))

(event `self.ReceiveEndPlay`
  (params (EndPlayReason :type "EEndPlayReason Enum" :default "Destroyed"))
  ;[1 1 1] Save the States
  (bind _returnvalue (`GameplayStatics.CreateSaveGameObject` "/Game/Blueprints/RSave.RSave_C"))
  (set `/Game/Blueprints/RSave.States` (`self.States`) _returnvalue)
  (`GameplayStatics.SaveGameToSlot` _returnvalue "Cube" (`self.Dimension`)))

(event `Init`
  (bind _returnvalue (/ 5.0 (`KismetMathLibrary.Conv_IntToDouble` (* (+ (`/Game/Blueprints/GI_Cube.Difficulty` (cast `/Game/Blueprints/GI_Cube` (`GameplayStatics.GetGameInstance`) :!pure true)) 1) 10))))
  (`self.DisableInput` (`GameplayStatics.GetPlayerController` 0))
  (`Timeline|InitTimeline`
    (:`Update`
      (`KismetSystemLibrary.Delay` _returnvalue)
      (`self.RandomRot`))
    (:`Finished`
      (`KismetSystemLibrary.Delay` _returnvalue)
      (`self.EnableInput` null)
      (`self.Ready?`)
      (set `self.Moves` 0))))

(fn `Check Faces`
  (returns (`Return State` :type String) (Solved :type Boolean))
  (locals (State :type String) (`Solved?` :type Boolean :default true) (`Temp Face` :type Integer :default 0))
  (for _array_element (`self.FaceCheckCollisions`)
    (`|ExecutionSequence`
      (:`then_0`
        (goto _label :!via `Reset`))
      (:`then_1`
        (for _array_element_2 (`PrimitiveComponent.GetOverlappingComponents` _array_element)
          (if (`ActorComponent.ComponentHasTag` _array_element_2 "Side")
            (bind _ascuboid (cast `/Game/Blueprints/Cuboid` (`ActorComponent.GetOwner` _array_element_2)))
            (bind _asstatic_mesh_component (cast `StaticMeshComponent` _array_element_2))
            (`|ExecutionSequence`
              (:`then_0`
                (bind _returnvalue (`KismetArrayLibrary.Array_Find` (`/Game/Blueprints/Cuboid.Faces` _ascuboid) _asstatic_mesh_component))
                (set `local.State` (`KismetStringLibrary.Concat_StrStr` (`local.State`) (`KismetStringLibrary.Conv_IntToString` _returnvalue))))
              (:`then_1`
                (`/Engine/EditorBlueprintResources/StandardMacros.DoOnce` true :!label _label
                  (:`Completed`
                    (set `local.Temp Face` _returnvalue))))
              (:`then_2`
                (if (`local.Solved?`)
                  (if (not (== _returnvalue (`local.Temp Face`)))
                    (set `local.Solved?` false))))))))))
  (return (`local.State`) (`local.Solved?`)))

(fn `CommonColliders`
  (params (`Colliders 1` :type "Array of PrimitiveComponent Object Reference") (`Colliders 2` :type "Array of PrimitiveComponent Object Reference"))
  (returns (ReturnValue :type Boolean) (Component :type "PrimitiveComponent Object Reference"))
  (for _array_element `Colliders 1`
    (for _array_element_2 `Colliders 2`
      (if (and (== _array_element _array_element_2) (`ActorComponent.ComponentHasTag` _array_element_2 "Rotator"))
        (return true _array_element_2))))
  (return false null))

(fn `GetAxisVector`
  (params (Axis :type "/Game/Blueprints/E_Axis Enum" :default "NewEnumerator0") (InVec :type "Vector Structure") (Value :type "Float (single-precision)"))
  (returns (OutVec :type "Vector Structure") (`Out Size` :type "Vector Structure"))
  (bind _x (.x InVec))
  (bind _y (.y InVec))
  (bind _z (.z InVec))
  (bind _returnvalue (* (`self.Size`) (/ (`self.Dimension`) 2.1)))
  (return (select `/Game/Blueprints/E_Axis` Axis :`NewEnumerator0` (`KismetMathLibrary.MakeVector` (+ _x Value) _y _z) :`NewEnumerator1` (`KismetMathLibrary.MakeVector` _x (+ _y Value) _z) :`NewEnumerator2` (`KismetMathLibrary.MakeVector` _x _y (+ _z Value)) :!type "Vector Structure") (select `/Game/Blueprints/E_Axis` Axis :`NewEnumerator0` (`KismetMathLibrary.MakeVector` 5.0 _returnvalue _returnvalue) :`NewEnumerator1` (`KismetMathLibrary.MakeVector` _returnvalue 5.0 _returnvalue) :`NewEnumerator2` (`KismetMathLibrary.MakeVector` _returnvalue _returnvalue 5.0) :!type "Vector Structure")))

(fn `Outsside?`
  (params (Point :type "Vector Structure"))
  (returns (ReturnValue :type Boolean))
  (return (not (`KismetMathLibrary.IsPointInBox` Point (`SceneComponent.K2_GetComponentLocation` (`self.SpringArm`)) (`KismetMathLibrary.Conv_DoubleToVector` (* (`KismetMathLibrary.Conv_IntToDouble` (- (`self.Dimension`) 1)) (`self.Size`) 0.499999))))))

(fn `RandomRot`
  (locals (`Temp Rotator` :type "/Game/Blueprints/Rotator Object Reference"))
  (bind _output_get (set `local.Temp Rotator` (`KismetArrayLibrary.Array_Random` (select `int` (`KismetMathLibrary.RandomInteger` 3) :`0` (`self.XRotators`) :`1` (`self.YRotators`) :`2` (`self.ZRotator`)))))
  (`/Engine/EditorBlueprintResources/StandardMacros.IsValid` _output_get
    (:`Is Valid`
      (`/Game/Blueprints/Rotator.InstantRotate` _output_get (`KismetMathLibrary.RandomBool`) false))))

(fn `RandomRotSlow`
  (locals (`Temp Rotator` :type "/Game/Blueprints/Rotator Object Reference"))
  (bind _output_get (set `local.Temp Rotator` (`KismetArrayLibrary.Array_Random` (select `int` (`KismetMathLibrary.RandomInteger` 3) :`0` (`self.XRotators`) :`1` (`self.YRotators`) :`2` (`self.ZRotator`)))))
  (`/Engine/EditorBlueprintResources/StandardMacros.IsValid` _output_get
    (:`Is Valid`
      (`/Game/Blueprints/Rotator.Rotate` _output_get (`KismetMathLibrary.RandomBool`) 1.0 false))))

(fn `UserConstructionScript`)