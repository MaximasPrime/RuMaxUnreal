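; Cuboid is one coloured piece of a Rubik's-style cube (RCube), destroyed along with it.
; The construction script colours its six faces with dynamic material instances.
; After a short delay on BeginPlay, a capsule trace toward RCube's spring arm finds an inward "Side" face, and short per-face line traces, ignoring rotators, find faces touching neighbours.
; Those hidden faces turn grey and lose their component tags.
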(event `self.ReceiveBeginPlay`
  (bind _rotators (`self.Rotators`))
  (bind _rcube (`self.RCube`))
  (set `self.Size` (`KismetMathLibrary.FTrunc` (`/Game/Blueprints/RCube.Size` _rcube)))
  (`KismetSystemLibrary.Delay` 0.2)
  (`KismetArrayLibrary.Array_Append` _rotators (`/Game/Blueprints/RCube.XRotators` _rcube))
  (`KismetArrayLibrary.Array_Append` _rotators (`/Game/Blueprints/RCube.YRotators` _rcube))
  (`KismetArrayLibrary.Array_Append` _rotators (`/Game/Blueprints/RCube.ZRotator` _rcube))
  ;[1 1 1] Make all inward faces Grey
  (`|ExecutionSequence`
    (:`then_0`
      (bind (_outhit _returnvalue) (`KismetSystemLibrary.CapsuleTraceSingle` :`Start` (`SceneComponent.K2_GetComponentLocation` (`self.Scene`)) :`End` (`SceneComponent.K2_GetComponentLocation` (`/Game/Blueprints/RCube.SpringArm` (`self.RCube`))) :`Radius` 20.0 :`HalfHeight` 20.0 :`TraceChannel` "TraceTypeQuery1" :`bIgnoreSelf` false))
      (if _returnvalue
        (bind (_bblockinghit _binitialoverlap _time _distance _location _impactpoint _normal _impactnormal _physmat _hitactor _hitcomponent) (`GameplayStatics.BreakHitResult` _outhit))
        (if (`ActorComponent.ComponentHasTag` _hitcomponent "Side")
          (bind _returnvalue_2 (`PrimitiveComponent.CreateDynamicMaterialInstance` _hitcomponent 0 "/Game/Visuals/M_ColourMat.M_ColourMat" "None"))
          (`MaterialInstanceDynamic.SetVectorParameterValue` _returnvalue_2 "Colour" (struct :`R` 0.109375 :`G` 0.109375 :`B` 0.109375 :`A` 1.0))
          (set `ActorComponent.ComponentTags` (`|MakeArray`) _hitcomponent))))
    (:`then_1`
      ;[1 1 1] Make faces Grey which has toucing cube face
      (for _array_element (`self.Faces`)
        (bind _returnvalue_3 (`SceneComponent.K2_GetComponentLocation` _array_element))
        (bind (_outhit_2 _returnvalue_4) (`KismetSystemLibrary.LineTraceSingle` _returnvalue_3 (+ _returnvalue_3 (* (`SceneComponent.GetUpVector` _array_element) (/ (`self.Size`) 4))) "TraceTypeQuery1" true (`self.Rotators`)))
        (if _returnvalue_4
          (set `ActorComponent.ComponentTags` (`|MakeArray`) _array_element)
          (bind _returnvalue_5 (`PrimitiveComponent.CreateDynamicMaterialInstance` _array_element 0 "/Game/Visuals/M_ColourMat.M_ColourMat" "None"))
          (`MaterialInstanceDynamic.SetVectorParameterValue` _returnvalue_5 "Colour" (struct :`R` 0.109375 :`G` 0.109375 :`B` 0.109375 :`A` 1.0)))))
    (:`then_2`
      (add `self.OnDestroyed` (`self.RCube`) (delegate `OnDestroyed_Event_0`)))))

(event `OnDestroyed_Event_0` :!signature `self.OnDestroyed`
  (params (DestroyedActor :type "Actor Object Reference"))
  ;[1 1 1] Make all inward faces Grey
  (`self.K2_DestroyActor`))

(fn `SetFaceColour`
  (params (Element :type Integer) (Colour :type "LinearColor Structure"))
  (bind _returnvalue (`PrimitiveComponent.CreateDynamicMaterialInstance` (`|GetArrayItem` (`self.Faces`) Element) 0 "/Game/Visuals/M_ColourMat.M_ColourMat" "None"))
  (`MaterialInstanceDynamic.SetVectorParameterValue` _returnvalue "Colour" Colour))

(fn `UserConstructionScript`
  (set `self.Faces` (`|MakeArray` (`self.1`) (`self.2`) (`self.3`) (`self.4`) (`self.5`) (`self.6`)))
  (for (_array_element _array_index) (`self.Colours`)
    (`self.SetFaceColour` _array_index _array_element)))